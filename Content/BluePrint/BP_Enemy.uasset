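; BP_Enemy is an enemy that chases the first player character.
; Each Tick it feeds the vector from its own location to the player into AddMovementInput, steering straight at them with no pathfinding, range check or normalization.
; Unconnected nodes for randomized forward movement and yaw rotation never run, and the Speed variable is unused.
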(event `self.ReceiveTick`
  (params (DeltaSeconds :type "Float (single-precision)"))
  (`self.AddMovementInput` (- (`self.K2_GetActorLocation` (`GameplayStatics.GetPlayerCharacter` 0)) (`self.K2_GetActorLocation`))))

(fn `UserConstructionScript`)